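; BP_TrackGate is a time trial checkpoint gate that advances a player through the track in order.
; On overlap it gets the actor's instigator BP_TimeTrialPlayerController and acts only if this gate is that controller's TargetGate.
; It then sets TargetGate to its linked NextMarker and, if flagged as the finish line, increments the lap count.
; The construction script replaces the actor's tags with Finish or None according to that flag.
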(event EventBeginPlay)

(event Collision|EventActorBeginOverlap
  (params (OtherActor :type Actor%20Object%20Reference))
  (bind _returnvalue (Game|GetInstigatorController OtherActor))
  (Utilities|IsValid _returnvalue
    (:Is%20Valid
      (bind _asbp_time_trial_player_controller (Utilities|Casting|CastToBP_TimeTrialPlayerController _returnvalue))
      (if (== (Variables|/Game/Variant_Timetrial/Blueprints/BP_TimeTrialPlayerController.BP_TimeTrialPlayerController_C|GetTargetGate _asbp_time_trial_player_controller) self)
        (Variables|/Game/Variant_Timetrial/Blueprints/BP_TimeTrialPlayerController.BP_TimeTrialPlayerController_C|SetTargetGate _asbp_time_trial_player_controller (Variables|Default|GetNext%20Marker))
        (if (Variables|Default|GetIs%20Finish%20Line)
          (Default|IncrementLapCount _asbp_time_trial_player_controller))))))

(event EventTick
  (params (DeltaSeconds :type Float%20%28single-precision%29)))

(fn ConstructionScript
  (Variables|Default|SetTags (Utilities|Array|MakeArray (select (Variables|Default|GetIs%20Finish%20Line) "Finish" "None"))))